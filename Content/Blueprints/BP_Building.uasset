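; BP_Building is a building actor that visibly grows through two construction phases as wood and stone resources accumulate.
; BeginPlay shows only the Base component and hides Phase1 and Phase2.
; Tick checks WoodResources and StoneResources against a lower and a higher threshold, revealing each phase once and latching it with a boolean flag.
; Nothing here changes the resource counts, and revealed phases are never hidden again.
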(event EventBeginPlay
  (Rendering|SetVisibility (Variables|Default|GetPhase%201) false true)
  (Rendering|SetVisibility (Variables|Default|GetPhase%202) false true)
  (Rendering|SetVisibility (Variables|Default|GetBase) true false))

(event EventTick
  (params (DeltaSeconds :type Float%20%28single-precision%29))
  (if (and (not (Variables|Default|GetIsPhase1)) (and (>= (Variables|Default|GetWoodResources) 25) (>= (Variables|Default|GetStoneResources) 25)))
    (Rendering|SetVisibility (Variables|Default|GetPhase%201) true true)
    (Variables|Default|SetIsPhase1 true)
    (elif (and (not (Variables|Default|GetIsPhase2)) (and (>= (Variables|Default|GetWoodResources) 75) (>= (Variables|Default|GetStoneResources) 75)))
      (Rendering|SetVisibility (Variables|Default|GetPhase%202) true true)
      (Variables|Default|SetIsPhase2 true))))

(fn ConstructionScript)